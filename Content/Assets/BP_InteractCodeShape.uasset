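; Shape-code puzzle actor that generates a random three-shape code and can open a linked BP_LockableDoor.
; Shortly after BeginPlay, GetCode picks random Wand or WandRaum2 actors, re-rolling duplicates by display name, storing their hint shapes as RightSlots and pictures on three BP_Hint actors.
; ChangeSlot functions set each display mesh and scale from its current Slot value.
; OpenDoor hides the door cube and disables collision; no code check exists here.
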(event EventBeginPlay
  (Utilities|FlowControl|Delay 0.2)
  (CallFunction|GetCode)
  (CallFunction|ChangeSlot1)
  (CallFunction|ChangeSlot2)
  (CallFunction|ChangeSlot3))

(event Collision|EventActorBeginOverlap
  (params (OtherActor :type Actor%20Object%20Reference)))

(event EventTick
  (params (DeltaSeconds :type Float%20%28single-precision%29)))

(fn ConstructionScript)

(fn ChangeSlot1
  (bind _color1 (Variables|Default|GetColor1))
  (bind _slot1 (Variables|Default|GetSlot1))
  (bind _color1_2 (Variables|Default|GetColor1))
  (if (Utilities|Enum|Equal(Enum) _slot1 "Cube")
    (Development|PrintString "0")
    (Components|StaticMesh|SetStaticMesh (Variables|Default|GetColor1) "/Game/LevelPrototyping/Meshes/SM_Cube.SM_Cube")
    (elif (Utilities|Enum|Equal(Enum) _slot1 "Sphere")
      (Development|PrintString "1")
      (Components|StaticMesh|SetStaticMesh _color1_2 "/Game/FPWeapon/Mesh/FirstPersonProjectileMesh.FirstPersonProjectileMesh")
      (Transformation|SetWorldScale3D _color1_2 (/ (Transformation|GetWorldScale _color1_2) "2.000000,2.000000,2.000000"))
      (elif (Utilities|Enum|Equal(Enum) _slot1 "Ramp")
        (Development|PrintString "2")
        (Components|StaticMesh|SetStaticMesh (Variables|Default|GetColor1) "/Game/LevelPrototyping/Meshes/SM_Ramp.SM_Ramp")
        (else
          (Development|PrintString "3")
          (Components|StaticMesh|SetStaticMesh _color1 "/Game/LevelPrototyping/Meshes/SM_Cylinder.SM_Cylinder")
          (Transformation|SetWorldScale3D _color1 (Transformation|GetWorldScale (Variables|Default|GetOrginalScale))))))))

(fn ChangeSlot2
  (bind _slot2 (Variables|Default|GetSlot2))
  (bind _color2 (Variables|Default|GetColor2))
  (if (Utilities|Enum|Equal(Enum) _slot2 "Cube")
    (Development|PrintString "0")
    (Components|StaticMesh|SetStaticMesh _color2 "/Game/LevelPrototyping/Meshes/SM_Cube.SM_Cube")
    (elif (Utilities|Enum|Equal(Enum) _slot2 "Sphere")
      (Development|PrintString "1")
      (Components|StaticMesh|SetStaticMesh _color2 "/Game/FPWeapon/Mesh/FirstPersonProjectileMesh.FirstPersonProjectileMesh")
      (Transformation|SetWorldScale3D _color2 (/ (Transformation|GetWorldScale (Variables|Default|GetOrginalScale)) "2.000000,2.000000,2.000000"))
      (elif (Utilities|Enum|Equal(Enum) _slot2 "Ramp")
        (Development|PrintString "2")
        (Components|StaticMesh|SetStaticMesh _color2 "/Game/LevelPrototyping/Meshes/SM_Ramp.SM_Ramp")
        (else
          (Development|PrintString "3")
          (Components|StaticMesh|SetStaticMesh _color2 "/Game/LevelPrototyping/Meshes/SM_Cylinder.SM_Cylinder")
          (Transformation|SetWorldScale3D _color2 (Transformation|GetWorldScale (Variables|Default|GetOrginalScale))))))))

(fn ChangeSlot3
  (bind _slot3 (Variables|Default|GetSlot3))
  (bind _color3 (Variables|Default|GetColor3))
  (if (Utilities|Enum|Equal(Enum) _slot3 "Cube")
    (Development|PrintString "0")
    (Components|StaticMesh|SetStaticMesh _color3 "/Game/LevelPrototyping/Meshes/SM_Cube.SM_Cube")
    (elif (Utilities|Enum|Equal(Enum) _slot3 "Sphere")
      (Development|PrintString "1")
      (Components|StaticMesh|SetStaticMesh _color3 "/Game/FPWeapon/Mesh/FirstPersonProjectileMesh.FirstPersonProjectileMesh")
      (Transformation|SetWorldScale3D _color3 (/ (Transformation|GetWorldScale (Variables|Default|GetOrginalScale)) "2.000000,2.000000,2.000000"))
      (elif (Utilities|Enum|Equal(Enum) _slot3 "Ramp")
        (Development|PrintString "2")
        (Components|StaticMesh|SetStaticMesh _color3 "/Game/LevelPrototyping/Meshes/SM_Ramp.SM_Ramp")
        (else
          (Development|PrintString "3")
          (Components|StaticMesh|SetStaticMesh _color3 "/Game/LevelPrototyping/Meshes/SM_Cylinder.SM_Cylinder")
          (Transformation|SetWorldScale3D _color3 (Transformation|GetWorldScale (Variables|Default|GetOrginalScale))))))))

(fn OpenDoor
  (bind _asbp_lockable_door (Utilities|Casting|CastToBP_LockableDoor (Variables|Default|GetDoor)))
  (Collision|SetCollisionEnabled (Variables|/Game/Assets/BP_LockableDoor.BP_LockableDoor_C|GetCube _asbp_lockable_door) "NoCollision")
  (Rendering|SetVisibility (Variables|/Game/Assets/BP_LockableDoor.BP_LockableDoor_C|GetCube _asbp_lockable_door) false false))

(fn GetCode
  (if (> (Math|Random|RandomInteger 2) 0)
    (bind _outactors (Actor|GetAllActorsOfClass "/Game/Assets/Wand.Wand_C"))
    (bind _output_get (Variables|Default|SetExamplePawn (Utilities|Array|Get(acopy) _outactors (Math|Random|RandomInteger (Utilities|Array|Length _outactors)))))
    (bind _aswand (Utilities|Casting|CastToWand _output_get))
    (switch int (Variables|/Game/Assets/BP_HintCube.BP_HintCube_C|GetIntMesh (Variables|/Game/Assets/Wand.Wand_C|GetHintCube _aswand))
      (:0
        (bind _output_get_2 (Variables|Default|SetRightSlot1 "NewEnumerator4"))
        (Development|PrintString (Utilities|String|EnumtoString _output_get_2)))
      (:1
        (bind _output_get_3 (Variables|Default|SetRightSlot1 "NewEnumerator5"))
        (Development|PrintString (Utilities|String|EnumtoString _output_get_3)))
      (:2
        (bind _output_get_4 (Variables|Default|SetRightSlot1 "NewEnumerator6"))
        (Development|PrintString (Utilities|String|EnumtoString _output_get_4))))
    (bind _asbp_hint (Utilities|Casting|CastToBP_Hint (Variables|Default|GetFirstHint))
      (:then
        _)
      (:CastFailed
        _))
    (Development|PrintString "1")
    (Default|SetPicture _asbp_hint (Variables|/Game/Assets/Wand.Wand_C|GetHintPic _aswand))
    (else
      (bind _outactors_2 (Actor|GetAllActorsOfClass "/Game/Assets/WandRaum2.WandRaum2_C"))
      (bind _output_get_5 (Variables|Default|SetExamplePawn (Utilities|Array|Get(acopy) _outactors_2 (Math|Random|RandomInteger (Utilities|Array|Length _outactors_2)))))
      (bind _aswand_raum_2 (Utilities|Casting|CastToWandRaum2 _output_get_5))
      (switch int (Variables|/Game/Assets/BP_HintCube.BP_HintCube_C|GetIntMesh (Variables|/Game/Assets/WandRaum2.WandRaum2_C|GetHintCube _aswand_raum_2))
        (:0
          (bind _output_get_6 (Variables|Default|SetRightSlot1 "NewEnumerator4"))
          (Development|PrintString (Utilities|String|EnumtoString _output_get_6)))
        (:1
          (bind _output_get_7 (Variables|Default|SetRightSlot1 "NewEnumerator5"))
          (Development|PrintString (Utilities|String|EnumtoString _output_get_7)))
        (:2
          (bind _output_get_8 (Variables|Default|SetRightSlot1 "NewEnumerator6"))
          (Development|PrintString (Utilities|String|EnumtoString _output_get_8))))
      (bind _asbp_hint_2 (Utilities|Casting|CastToBP_Hint (Variables|Default|GetFirstHint))
        (:then
          _)
        (:CastFailed
          _))
      (Development|PrintString "2")
      (Default|SetPicture _asbp_hint_2 (Variables|/Game/Assets/WandRaum2.WandRaum2_C|GetHintPic _aswand_raum_2))))
  (Development|PrintString "2.")
  (if (> (Math|Random|RandomInteger 2) 0) :!label _label
    (bind _outactors_3 (Actor|GetAllActorsOfClass "/Game/Assets/Wand.Wand_C"))
    (bind _output_get_9 (Variables|Default|SetExamplePawn2 (Utilities|Array|Get(acopy) _outactors_3 (Math|Random|RandomInteger (Utilities|Array|Length _outactors_3)))))
    (bind _aswand_2 (Utilities|Casting|CastToWand _output_get_9))
    (switch int (Variables|/Game/Assets/BP_HintCube.BP_HintCube_C|GetIntMesh (Variables|/Game/Assets/Wand.Wand_C|GetHintCube _aswand_2))
      (:0
        (bind _output_get_10 (Variables|Default|SetRightSlot2 "NewEnumerator4"))
        (Development|PrintString (Utilities|String|EnumtoString _output_get_10)))
      (:1
        (bind _output_get_11 (Variables|Default|SetRightSlot2 "NewEnumerator5"))
        (Development|PrintString (Utilities|String|EnumtoString _output_get_11)))
      (:2
        (bind _output_get_12 (Variables|Default|SetRightSlot2 "NewEnumerator6"))
        (Development|PrintString (Utilities|String|EnumtoString _output_get_12))))
    (bind _asbp_hint_3 (Utilities|Casting|CastToBP_Hint (Variables|Default|GetSecoundHint)))
    (Default|SetPicture _asbp_hint_3 (Variables|/Game/Assets/Wand.Wand_C|GetHintPic _aswand_2))
    (else
      (bind _outactors_4 (Actor|GetAllActorsOfClass "/Game/Assets/WandRaum2.WandRaum2_C"))
      (bind _output_get_13 (Variables|Default|SetExamplePawn2 (Utilities|Array|Get(acopy) _outactors_4 (Math|Random|RandomInteger (Utilities|Array|Length _outactors_4)))))
      (bind _aswand_raum_2_2 (Utilities|Casting|CastToWandRaum2 _output_get_13))
      (switch int (Variables|/Game/Assets/BP_HintCube.BP_HintCube_C|GetIntMesh (Variables|/Game/Assets/WandRaum2.WandRaum2_C|GetHintCube _aswand_raum_2_2))
        (:0
          (bind _output_get_14 (Variables|Default|SetRightSlot2 "NewEnumerator4"))
          (Development|PrintString (Utilities|String|EnumtoString _output_get_14)))
        (:1
          (bind _output_get_15 (Variables|Default|SetRightSlot2 "NewEnumerator5"))
          (Development|PrintString (Utilities|String|EnumtoString _output_get_15)))
        (:2
          (bind _output_get_16 (Variables|Default|SetRightSlot2 "NewEnumerator6"))
          (Development|PrintString (Utilities|String|EnumtoString _output_get_16))))
      (bind _asbp_hint_4 (Utilities|Casting|CastToBP_Hint (Variables|Default|GetSecoundHint)))
      (Default|SetPicture _asbp_hint_4 (Variables|/Game/Assets/WandRaum2.WandRaum2_C|GetHintPic _aswand_raum_2_2))))
  (if (Utilities|Enum|Equal(Enum) (Utilities|GetDisplayName (Variables|Default|GetExamplePawn)) (Utilities|GetDisplayName (Variables|Default|GetExamplePawn2)))
    (goto _label)
    (else
      (if (> (Math|Random|RandomInteger 2) 0) :!label _label_2
        (bind _outactors_5 (Actor|GetAllActorsOfClass "/Game/Assets/Wand.Wand_C"))
        (bind _output_get_17 (Variables|Default|SetExamplePawn3 (Utilities|Array|Get(acopy) _outactors_5 (Math|Random|RandomInteger (Utilities|Array|Length _outactors_5)))))
        (bind _aswand_3 (Utilities|Casting|CastToWand _output_get_17))
        (switch int (Variables|/Game/Assets/BP_HintCube.BP_HintCube_C|GetIntMesh (Variables|/Game/Assets/Wand.Wand_C|GetHintCube _aswand_3))
          (:0
            (bind _output_get_18 (Variables|Default|SetRightSlot3 "NewEnumerator4"))
            (Development|PrintString (Utilities|String|EnumtoString _output_get_18)))
          (:1
            (bind _output_get_19 (Variables|Default|SetRightSlot3 "NewEnumerator5"))
            (Development|PrintString (Utilities|String|EnumtoString _output_get_19)))
          (:2
            (bind _output_get_20 (Variables|Default|SetRightSlot3 "NewEnumerator6"))
            (Development|PrintString (Utilities|String|EnumtoString _output_get_20))))
        (bind _asbp_hint_5 (Utilities|Casting|CastToBP_Hint (Variables|Default|GetThirdHint)))
        (Default|SetPicture _asbp_hint_5 (Variables|/Game/Assets/Wand.Wand_C|GetHintPic _aswand_3))
        (else
          (bind _outactors_6 (Actor|GetAllActorsOfClass "/Game/Assets/WandRaum2.WandRaum2_C"))
          (bind _output_get_21 (Variables|Default|SetExamplePawn3 (Utilities|Array|Get(acopy) _outactors_6 (Math|Random|RandomInteger (Utilities|Array|Length _outactors_6)))))
          (bind _aswand_raum_2_3 (Utilities|Casting|CastToWandRaum2 _output_get_21))
          (switch int (Variables|/Game/Assets/BP_HintCube.BP_HintCube_C|GetIntMesh (Variables|/Game/Assets/WandRaum2.WandRaum2_C|GetHintCube _aswand_raum_2_3))
            (:0
              (bind _output_get_22 (Variables|Default|SetRightSlot3 "NewEnumerator4"))
              (Development|PrintString (Utilities|String|EnumtoString _output_get_22)))
            (:1
              (bind _output_get_23 (Variables|Default|SetRightSlot3 "NewEnumerator5"))
              (Development|PrintString (Utilities|String|EnumtoString _output_get_23)))
            (:2
              (bind _output_get_24 (Variables|Default|SetRightSlot3 "NewEnumerator6"))
              (Development|PrintString (Utilities|String|EnumtoString _output_get_24))))
          (bind _asbp_hint_6 (Utilities|Casting|CastToBP_Hint (Variables|Default|GetThirdHint)))
          (Default|SetPicture _asbp_hint_6 (Variables|/Game/Assets/WandRaum2.WandRaum2_C|GetHintPic _aswand_raum_2_3))))
      (if (or (Utilities|Enum|Equal(Enum) (Utilities|GetDisplayName (Variables|Default|GetExamplePawn)) (Utilities|GetDisplayName (Variables|Default|GetExamplePawn3))) (Utilities|Enum|Equal(Enum) (Utilities|GetDisplayName (Variables|Default|GetExamplePawn2)) (Utilities|GetDisplayName (Variables|Default|GetExamplePawn3))))
        (goto _label_2)))))