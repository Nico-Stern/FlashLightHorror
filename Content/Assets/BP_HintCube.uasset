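; BP_HintCube is a hint prop that randomizes its color and shape when play begins.
; PickColor applies a blue, yellow or red material and records the choice in IntColor.
; PichMesh keeps the default mesh, swaps to a half-scale projectile mesh, or swaps to a ramp with halved world Z, recording the choice in IntMesh.
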(event EventBeginPlay
  (CallFunction|PickColor)
  (CallFunction|PichMesh))

(event Collision|EventActorBeginOverlap
  (params (OtherActor :type Actor%20Object%20Reference)))

(event EventTick
  (params (DeltaSeconds :type Float%20%28single-precision%29)))

(fn ConstructionScript)

(fn PickColor
  (bind _cube (Variables|Default|GetCube))
  (switch int (Math|Random|RandomInteger 3)
    (:0
      (Rendering|Material|SetMaterial _cube 0 "/Game/Material/MI_ColorBlue.MI_ColorBlue")
      (Variables|Default|SetIntColor 0))
    (:1
      (Rendering|Material|SetMaterial _cube 0 "/Game/Material/MI_ColorYellow.MI_ColorYellow")
      (Variables|Default|SetIntColor 1))
    (:2
      (Rendering|Material|SetMaterial _cube 0 "/Game/Material/MI_ColorRed.MI_ColorRed")
      (Variables|Default|SetIntColor 2))))

(fn PichMesh
  (bind _cube (Variables|Default|GetCube))
  (bind _cube_2 (Variables|Default|GetCube))
  (switch int (Math|Random|RandomInteger 3)
    (:0
      (Variables|Default|SetIntMesh 0))
    (:1
      (Transformation|SetWorldScale3D _cube_2 (/ (Transformation|GetWorldScale _cube_2) "2.000000,2.000000,2.000000"))
      (Components|StaticMesh|SetStaticMesh _cube "/Game/FPWeapon/Mesh/FirstPersonProjectileMesh.FirstPersonProjectileMesh")
      (Variables|Default|SetIntMesh 1))
    (:2
      (Transformation|SetWorldLocation _cube (/ (Transformation|GetWorldLocation _cube) "1.000000,1.000000,2.000000") false false)
      (Components|StaticMesh|SetStaticMesh _cube "/Game/LevelPrototyping/Meshes/SM_Ramp.SM_Ramp")
      (Variables|Default|SetIntMesh 2))))