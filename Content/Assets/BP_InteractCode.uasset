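; Colour-code lock puzzle that builds a random three-colour solution from the level's Wand actors and can open a linked BP_LockableDoor.
; Shortly after BeginPlay, GetCode re-rolls until it has three distinct Wands, stores their HintCube colours as RightSlot values and shows their pictures on three BP_Hint actors.
; ChangeSlot functions recolour each display from its slot value.
; OpenDoor hides the door cube and disables its collision; no comparison or caller appears here.
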(event EventBeginPlay
  (Utilities|FlowControl|Delay 0.2)
  (CallFunction|GetCode))

(event Collision|EventActorBeginOverlap
  (params (OtherActor :type Actor%20Object%20Reference)))

(event EventTick
  (params (DeltaSeconds :type Float%20%28single-precision%29)))

(fn ConstructionScript)

(fn ChangeSlot1
  (switch int (Math|Conversions|ToInteger(Byte) (Variables|Default|GetSlot1))
    (:0
      (Development|PrintString "0")
      (Rendering|Material|SetMaterial (Variables|Default|GetColor1) 0 "/Game/FPWeapon/Materials/BaseMaterial.BaseMaterial"))
    (:1
      (Development|PrintString "1")
      (Rendering|Material|SetMaterial (Variables|Default|GetColor1) 0 "/Game/Material/MI_ColorBlue.MI_ColorBlue"))
    (:2
      (Development|PrintString "2")
      (Rendering|Material|SetMaterial (Variables|Default|GetColor1) 0 "/Game/Material/MI_ColorYellow.MI_ColorYellow"))
    (:3
      (Development|PrintString "3")
      (Rendering|Material|SetMaterial (Variables|Default|GetColor1) 0 "/Game/Material/MI_ColorRed.MI_ColorRed"))))

(fn ChangeSlot2
  (bind _color2 (Variables|Default|GetColor2))
  (switch int (Math|Conversions|ToInteger(Byte) (Variables|Default|GetSlot2))
    (:0
      (Development|PrintString "0")
      (Rendering|Material|SetMaterial _color2 0 "/Game/FPWeapon/Materials/BaseMaterial.BaseMaterial"))
    (:1
      (Development|PrintString "1")
      (Rendering|Material|SetMaterial _color2 0 "/Game/Material/MI_ColorBlue.MI_ColorBlue"))
    (:2
      (Development|PrintString "2")
      (Rendering|Material|SetMaterial _color2 0 "/Game/Material/MI_ColorYellow.MI_ColorYellow"))
    (:3
      (Development|PrintString "3")
      (Rendering|Material|SetMaterial _color2 0 "/Game/Material/MI_ColorRed.MI_ColorRed"))))

(fn ChangeSlot3
  (bind _color3 (Variables|Default|GetColor3))
  (switch int (Math|Conversions|ToInteger(Byte) (Variables|Default|GetSlot3))
    (:0
      (Development|PrintString "0")
      (Rendering|Material|SetMaterial _color3 0 "/Game/FPWeapon/Materials/BaseMaterial.BaseMaterial"))
    (:1
      (Development|PrintString "1")
      (Rendering|Material|SetMaterial _color3 0 "/Game/Material/MI_ColorBlue.MI_ColorBlue"))
    (:2
      (Development|PrintString "2")
      (Rendering|Material|SetMaterial _color3 0 "/Game/Material/MI_ColorYellow.MI_ColorYellow"))
    (:3
      (Development|PrintString "3")
      (Rendering|Material|SetMaterial _color3 0 "/Game/Material/MI_ColorRed.MI_ColorRed"))))

(fn OpenDoor
  (bind _asbp_lockable_door (Utilities|Casting|CastToBP_LockableDoor (Variables|Default|GetDoor)))
  (Collision|SetCollisionEnabled (Variables|/Game/Assets/BP_LockableDoor.BP_LockableDoor_C|GetCube _asbp_lockable_door) "NoCollision")
  (Rendering|SetVisibility (Variables|/Game/Assets/BP_LockableDoor.BP_LockableDoor_C|GetCube _asbp_lockable_door) false false))

(fn GetCode
  (bind _outactors (Actor|GetAllActorsOfClass "/Game/Assets/Wand.Wand_C"))
  (bind _output_get (Variables|Default|SetExamplePawn (Utilities|Array|Get(acopy) _outactors (Math|Random|RandomInteger (Utilities|Array|Length _outactors)))))
  (bind _aswand (Utilities|Casting|CastToWand _output_get))
  (bind _output_get_2 (Variables|Default|SetExamplePawn2 (Utilities|Array|Get(acopy) _outactors (Math|Random|RandomInteger (Utilities|Array|Length _outactors))) :!label _label))
  (bind _aswand_2 (Utilities|Casting|CastToWand _output_get_2))
  (if (== _output_get _output_get_2)
    (goto _label)
    (else
      (bind _output_get_3 (Variables|Default|SetExamplePawn3 (Utilities|Array|Get(acopy) _outactors (Math|Random|RandomInteger (Utilities|Array|Length _outactors))) :!label _label_2))
      (bind _aswand_3 (Utilities|Casting|CastToWand _output_get_3))
      (if (or (== _output_get _output_get_3) (== _output_get_2 _output_get_3))
        (goto _label_2)
        (else
          (switch int (Variables|/Game/Assets/BP_HintCube.BP_HintCube_C|GetIntColor (Variables|/Game/Assets/Wand.Wand_C|GetHintCube _aswand))
            (:0
              (bind _output_get_4 (Variables|Default|SetRightSlot1 "NewEnumerator1"))
              (Development|PrintString (Utilities|String|EnumtoString _output_get_4)))
            (:1
              (bind _output_get_5 (Variables|Default|SetRightSlot1 "NewEnumerator2"))
              (Development|PrintString (Utilities|String|EnumtoString _output_get_5)))
            (:2
              (bind _output_get_6 (Variables|Default|SetRightSlot1 "NewEnumerator3"))
              (Development|PrintString (Utilities|String|EnumtoString _output_get_6))))
          (bind _asbp_hint (Utilities|Casting|CastToBP_Hint (Variables|Default|GetFirstHint)))
          (Default|SetPicture _asbp_hint (Variables|/Game/Assets/Wand.Wand_C|GetHintPic _aswand))
          (switch int (Variables|/Game/Assets/BP_HintCube.BP_HintCube_C|GetIntColor (Variables|/Game/Assets/Wand.Wand_C|GetHintCube _aswand_2))
            (:0
              (bind _output_get_7 (Variables|Default|SetRightSlot2 "NewEnumerator1"))
              (Development|PrintString (Utilities|String|EnumtoString _output_get_7)))
            (:1
              (bind _output_get_8 (Variables|Default|SetRightSlot2 "NewEnumerator2"))
              (Development|PrintString (Utilities|String|EnumtoString _output_get_8)))
            (:2
              (bind _output_get_9 (Variables|Default|SetRightSlot2 "NewEnumerator3"))
              (Development|PrintString (Utilities|String|EnumtoString _output_get_9))))
          (bind _asbp_hint_2 (Utilities|Casting|CastToBP_Hint (Variables|Default|GetSecoundHint)))
          (Default|SetPicture _asbp_hint_2 (Variables|/Game/Assets/Wand.Wand_C|GetHintPic _aswand_2))
          (switch int (Variables|/Game/Assets/BP_HintCube.BP_HintCube_C|GetIntColor (Variables|/Game/Assets/Wand.Wand_C|GetHintCube _aswand_3))
            (:0
              (bind _output_get_10 (Variables|Default|SetRightSlot3 "NewEnumerator1"))
              (Development|PrintString (Utilities|String|EnumtoString _output_get_10)))
            (:1
              (bind _output_get_11 (Variables|Default|SetRightSlot3 "NewEnumerator2"))
              (Development|PrintString (Utilities|String|EnumtoString _output_get_11)))
            (:2
              (bind _output_get_12 (Variables|Default|SetRightSlot3 "NewEnumerator3"))
              (Development|PrintString (Utilities|String|EnumtoString _output_get_12))))
          (bind _asbp_hint_3 (Utilities|Casting|CastToBP_Hint (Variables|Default|GetThirdHint)))
          (Default|SetPicture _asbp_hint_3 (Variables|/Game/Assets/Wand.Wand_C|GetHintPic _aswand_3)))))))